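; AI turret that sweeps for targets, aims and fires projectiles, and can be frozen or destroyed.
; A state machine (Searching, Idle, Attacking, Frozen) drives it: timelines handle the back-and-forth sweep and idle droop after a timeout, while Tick handles aiming and timed firing.
; SetTarget, with no caller in this graph, switches between attacking and searching unless frozen.
; BPFreezableComponent receives dynamic materials and triggers freeze state changes through a bound event.
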(event `self.ReceiveBeginPlay`
  ;[0.4491 0.8591 1] Initialise state
  (`self.ChangeState` "NewEnumerator1")
  ;[0.4491 0.8591 1] Set up freezing and bind to freeze event
  (`self.SetUpFreezableComponent`)
  (add `/Game/GPP/Blueprints/Components/BP_FreezableComponent.OnFrozenChanged` (`self.BP_FreezableComponent`) (delegate `OnFrozenChanged`)))

(event `OnFrozenChanged`
  (params (IsFrozen :type Boolean))
  ;[0.4491 0.8591 1] Set up freezing and bind to freeze event
  (if IsFrozen
    (`self.ChangeState` "NewEnumerator3")
    (else
      (`self.ChangeState` "NewEnumerator1"))))

(event `self.ReceiveDestroyed`
  ;[0.4491 0.8591 1] Set up freezing and bind to freeze event
  (remove `/Game/GPP/Blueprints/Components/BP_FreezableComponent.OnFrozenChanged` (`self.BP_FreezableComponent`) (delegate `OnFrozenChanged`)))

(event `self.ReceiveTick`
  (params (DeltaSeconds :type "Float (single-precision)"))
  ;[0.4491 0.8591 1] Handle state logic that requires ticks
  (switch `/Game/GPP/Blueprints/NPCs/AI_Turret/Blueprints/E_TurretState_Example` (`self.State`)
    (:`NewEnumerator1`
      (`self.Searching` DeltaSeconds))
    (:`NewEnumerator2`
      (`self.Attacking` DeltaSeconds))))

(event `Searching`
  (params (DeltaTime :type "Float (double-precision)"))
  ;[0.4491 0.8591 1] Searching - Logic
  ;;[0.4491 0.8591 1] Idle Countdown
  (bind _output_get (set `self.IdleTimer` (+ (`self.IdleTimer`) DeltaTime)))
  (if (> _output_get (`self.IdleTime`))
    (`|ExecutionSequence`
      (:`then_0`
        (`self.StopSearching`)
        (set `self.IdleTimer` 0.0))
      (:`then_1`
        (`self.ChangeState` "NewEnumerator0")))))

(event `Attacking`
  (params (DeltaTime :type "Float (double-precision)"))
  ;[0.4491 0.8591 1] Attacking State - Tick
  (if (`self.IsAbleToAttack`)
    (`|ExecutionSequence`
      (:`then_0`
        (`self.LookAtTarget`))
      (:`then_1`
        (`self.FireAtTarget` (* DeltaTime (`self.shoot_speed`)))))))

(event `StartSearchingFromCurrent`
  ;[0.4491 0.8591 1] Searching - Logic
  ;;[0.4491 0.8591 1] Handle search roation
  (bind (_direction _alpha) (`Timeline|SearchingTimeline` :!label _label)
    (:`Update`
      (`SceneComponent.K2_SetWorldRotation` (`self.Pivot`) (`KismetMathLibrary.RLerp` (`self.CurrentRotation`) (`self.TargetRotation`) _alpha) false false))
    (:`Finished`
      (`self.FinishedSeekingRotation`))))

(event `FinishedSeekingRotation`
  ;[0.4491 0.8591 1] Searching - Logic
  ;;[0.4491 0.8591 1] Reset after finished rotating
  (`self.FlipFlopRotations`)
  (`KismetSystemLibrary.Delay` 0.2)
  (`self.StartSearchingFromBeginning`))

(event `StartSearchingFromBeginning`
  ;[0.4491 0.8591 1] Searching - Logic
  ;;[0.4491 0.8591 1] Handle search roation
  (goto _label :!via `PlayFromStart`))

(event `Idle`
  (bind _startingrotation (`self.StartingRotation`))
  ;[0.4491 0.8591 1] Idle
  (bind (_direction _alpha) (`Timeline|Idle_Timeline` :!via `PlayFromStart`)
    (:`Update`
      (`SceneComponent.K2_SetWorldRotation` (`self.Pivot`) (`KismetMathLibrary.RLerp` _startingrotation (`KismetMathLibrary.MakeRotator` (.roll _startingrotation) -40.0 (.yaw _startingrotation)) _alpha) false false))))

(event `StopSearching`
  ;[0.4491 0.8591 1] Searching - Logic
  ;;[0.4491 0.8591 1] Handle search roation
  (goto _label :!via `Stop`))

(event `FlipFlopRotations`
  ;[0.4491 0.8591 1] Searching - Logic
  ;;[0.4491 0.8591 1] Flip flop rotations
  (set `self.TempRotation` (`self.TargetRotation`))
  (set `self.TargetRotation` (`self.CurrentRotation`))
  (set `self.CurrentRotation` (`self.TempRotation`)))

(event `self.Destroy`
  (params (Instigator :type "Actor Object Reference"))
  ;[0.4491 0.8591 1] Destroy - Damagable Interface
  (`self.K2_DestroyActor`))

(fn `ChangeState`
  (params (State :type "/Game/GPP/Blueprints/NPCs/AI_Turret/Blueprints/E_TurretState_Example Enum" :default "NewEnumerator0"))
  (bind (_startingrotation_roll _startingrotation_pitch _startingrotation_yaw) (`KismetMathLibrary.BreakRotator` (`self.StartingRotation`)))
  (bind (_startingrotation_roll_2 _startingrotation_pitch_2 _startingrotation_yaw_2) (`KismetMathLibrary.BreakRotator` (`self.StartingRotation`)))
  (bind _output_get (set `self.State` State))
  ;[0.4491 0.8591 1] Handle initial state logic
  (switch `/Game/GPP/Blueprints/NPCs/AI_Turret/Blueprints/E_TurretState_Example` _output_get
    (:`NewEnumerator0`
      (`self.SetStartingRotation`)
      (`self.Idle`))
    (:`NewEnumerator1`
      ;;[0.4491 0.8591 1] Set up rotation
      (`self.SetStartingRotation`)
      (bind _output_get_2 (set `self.MaxRotation` (`KismetMathLibrary.MakeRotator` _startingrotation_roll_2 _startingrotation_pitch_2 (+ _startingrotation_yaw_2 30.0))))
      (set `self.CurrentRotation` _output_get_2)
      (bind _output_get_3 (set `self.MinRotation` (`KismetMathLibrary.MakeRotator` _startingrotation_roll _startingrotation_pitch (- _startingrotation_yaw 30.0))))
      (set `self.TargetRotation` _output_get_3)
      (`self.StartSearchingFromCurrent`))
    (:`NewEnumerator3`
      (`self.StopSearching`))))

(fn `FireAtTarget`
  (params (DeltaTime :type "Float (double-precision)"))
  (bind (_returnvalue_location _returnvalue_rotation) (`KismetMathLibrary.BreakTransform` (`SceneComponent.K2_GetComponentToWorld` (`self.ProjectileSpawn`))))
  (bind _output_get (set `self.FireTimer` (+ (`self.FireTimer`) DeltaTime)))
  (if (>= _output_get (`self.FireRate`))
    (`|SpawnActorFromClass` "/Game/GPP/Blueprints/Obstacles/BP_SimpleProjectile.BP_SimpleProjectile_C" (`KismetMathLibrary.MakeTransform` _returnvalue_location _returnvalue_rotation) "AlwaysSpawn" "MultiplyWithRoot" null self)
    (set `self.FireTimer` 0.0)))

(fn `IsAbleToAttack`
  (returns (ReturnValue :type Boolean))
  (return (and (!= (`self.CurrentTarget`) null) (`|EnumEquality` (`self.State`) "NewEnumerator2"))))

(fn `LookAtTarget`
  (bind _pivot (`self.Pivot`))
  (bind _currenttarget (`self.CurrentTarget`))
  (`SceneComponent.K2_SetWorldRotation` _pivot (`KismetMathLibrary.FindLookAtRotation` (`SceneComponent.K2_GetComponentLocation` _pivot) (+ (`SceneComponent.K2_GetComponentLocation` (`Character.Mesh` _currenttarget)) (`KismetMathLibrary.MakeVector` 0.0 0.0 (`CapsuleComponent.GetScaledCapsuleHalfHeight` (`Character.CapsuleComponent` _currenttarget))))) false false))

(fn `SetStartingRotation`
  (set `self.StartingRotation` (`SceneComponent.K2_GetComponentRotation` (`self.Pivot`))))

(fn `SetTarget`
  (params (CurrentTarget :type "Character Object Reference"))
  (if (`|EnumInequality` (`self.State`) "NewEnumerator3")
    (bind _output_get (set `self.CurrentTarget` CurrentTarget))
    (if (!= _output_get null)
      (`self.ChangeState` "NewEnumerator2")
      (else
        (`self.ChangeState` "NewEnumerator1")))))

(fn `SetUpFreezableComponent`
  (bind _base (`self.Base`))
  (bind _turret (`self.Turret`))
  (bind _bp_freezablecomponent (`self.BP_FreezableComponent`))
  (`|ExecutionSequence`
    (:`then_0`
      ;[0.4491 0.8591 1] Set up dynamic material
      (bind _returnvalue (`KismetMaterialLibrary.CreateDynamicMaterialInstance` (`PrimitiveComponent.GetMaterial` _base 0)))
      (`PrimitiveComponent.SetMaterial` _base 0 _returnvalue))
    (:`then_1`
      (bind _returnvalue_2 (`KismetMaterialLibrary.CreateDynamicMaterialInstance` (`PrimitiveComponent.GetMaterial` _turret 0)))
      (`PrimitiveComponent.SetMaterial` _turret 0 _returnvalue_2))
    (:`then_2`
      ;[0.4491 0.8591 1] Init freeze component
      (`/Game/GPP/Blueprints/Components/BP_FreezableComponent.InitMaterial` _bp_freezablecomponent (`|MakeArray` _returnvalue _returnvalue_2))
      (`/Game/GPP/Blueprints/Components/BP_FreezableComponent.InitFreezeStatus` _bp_freezablecomponent))))

(fn `UserConstructionScript`)