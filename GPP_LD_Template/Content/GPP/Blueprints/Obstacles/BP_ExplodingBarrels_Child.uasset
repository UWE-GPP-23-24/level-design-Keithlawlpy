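; BP_ExplodingBarrels_Child is an exploding barrel obstacle variant that breaks a referenced wall when it goes off.
; After running the parent Tick, it polls each frame for a triggered state with an expired fuse timer.
; It then calls BreakWall on the wall actor, using the BarrelBroken flag to ensure this happens only once.
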(event `self.ReceiveTick`
  (params (DeltaSeconds :type "Float (single-precision)"))
  (`parent.ReceiveTick` DeltaSeconds)
  (if (and (not (`self.BarrelBroken`)) (and (<= (`self.FuseTimer`) 0.0) (`self.IsTriggered`)))
    (set `self.BarrelBroken` true)
    (`/Game/GPP/ExtrasAddon/BP_blastwall.BreakWall` (`self.WallActorRef`))))

(fn `UserConstructionScript`
  (`parent.UserConstructionScript`))